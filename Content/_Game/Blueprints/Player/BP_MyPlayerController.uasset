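; Player controller for a voxel world that lets the player place and remove blocks with the mouse.
; A Raycast helper traces from the camera along its view up to BlockDistance, with debug drawing enabled.
; When it hits a ChunkBase, right click places Stone and left click sets Air through ChunkWorldSubsystem's ModifyTargetVoxel.
; The hit normal offsets the target point outward for placing and inward for removing.
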(event `self.ReceiveBeginPlay`)

(event `Key|RightMouseButton`
  (params (Key :type "Key Structure"))
  (:`Pressed`
    (bind (_returnvalue _outhit) (`self.Raycast`))
    (if _returnvalue
      (bind (_bblockinghit _binitialoverlap _time _distance _location _impactpoint _normal _impactnormal _physmat _hitactor) (`GameplayStatics.BreakHitResult` _outhit))
      (cast `ChunkBase` _hitactor)
      (bind _returnvalue_2 (+ _location _normal))
      (`ChunkWorldSubsystem.ModifyTargetVoxel` (subsystem `ChunkWorldSubsystem`) (`VoxelFunctionLibrary.WorldToLocalBlockPosition` _returnvalue_2 (`self.ChunkSize`)) _returnvalue_2 "Stone"))))

(event `Key|LeftMouseButton`
  (params (Key :type "Key Structure"))
  (:`Pressed`
    (bind (_returnvalue _outhit) (`self.Raycast`))
    (if _returnvalue
      (bind (_bblockinghit _binitialoverlap _time _distance _location _impactpoint _normal _impactnormal _physmat _hitactor) (`GameplayStatics.BreakHitResult` _outhit))
      (cast `ChunkBase` _hitactor)
      (bind _returnvalue_2 (- _location _normal))
      (`ChunkWorldSubsystem.ModifyTargetVoxel` (subsystem `ChunkWorldSubsystem`) (`VoxelFunctionLibrary.WorldToLocalBlockPosition` _returnvalue_2 (`self.ChunkSize`)) _returnvalue_2 "Air"))))

(fn `Raycast`
  (returns (ReturnValue :type Boolean) (OutHit :type "HitResult Structure"))
  (bind _playercameramanager (`self.PlayerCameraManager`))
  (bind _returnvalue (`PlayerCameraManager.GetCameraLocation` _playercameramanager))
  (bind (_outhit _returnvalue_2) (`KismetSystemLibrary.LineTraceSingle` :`Start` _returnvalue :`End` (+ _returnvalue (* (`KismetMathLibrary.GetForwardVector` (`PlayerCameraManager.GetCameraRotation` _playercameramanager)) (`self.BlockDistance`))) :`TraceChannel` "TraceTypeQuery1" :`DrawDebugType` "ForDuration"))
  (return _returnvalue_2 _outhit))

(fn `UserConstructionScript`)